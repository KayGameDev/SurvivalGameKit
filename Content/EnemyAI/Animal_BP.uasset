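; Animal AI actor that wanders, takes sword hits from the Ash character and drops loot on death.
; Tick uses a Delay and IsMoving flag to roam to random reachable points; seeing the player starts a self-repeating random move loop, not a chase.
; Sword capsule overlaps during SlashSword reduce Health until Death spawns BP_Loot and destroys it.
; TakeDamage only spawns an explosion effect and runs on BeginPlay, not on hits.
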(event OnSeePawn(PawnSensing)
  (params (Pawn :type Pawn%20Object%20Reference))
  (Utilities|Casting|CastToBP_EBS_AshCharacter Pawn)
  (Variables|Default|SetIsMoving true)
  (AI|AIMoveTo self (.RandomLocation (AI|Navigation|GetRandomReachablePointinRadius (Transformation|GetActorLocation) 1e+03 0 0)) 0 5.0 false :!label _label
    (:OnSuccess
      _)
    (:OnFail
      _))
  (Utilities|FlowControl|Delay 0.5)
  (goto _label))

(event OnComponentBeginOverlap(CapsuleComponent)
  (params (OverlappedComponent :type Primitive%20Component%20Object%20Reference) (OtherActor :type Actor%20Object%20Reference) (OtherComp :type Primitive%20Component%20Object%20Reference) (OtherBodyIndex :type Integer) (bFromSweep :type Boolean) (SweepResult :type Hit%20Result%20Structure%20%28by%20ref%29))
  (Utilities|Casting|CastToWeapon_Ash_Sword OtherActor)
  (bind _asbp_ebs_ash_character (Utilities|Casting|CastToBP_EBS_AshCharacter (Game|GetPlayerCharacter 0)))
  (if (Variables|/Game/BP_EBS_AshCharacter.BP_EBS_AshCharacter_C|GetSlashSword _asbp_ebs_ash_character)
    (Development|PrintString "Hit with sword")
    (bind _output_get (Variables|Default|SetHealth (- (Variables|Default|GetHealth) 0.25)))
    (if (<= _output_get 0.0)
      (CallFunction|Death))))

(event EventBeginPlay
  (CallFunction|TakeDamage))

(event Collision|EventActorBeginOverlap
  (params (OtherActor :type Actor%20Object%20Reference)))

(event EventTick
  (params (DeltaSeconds :type Float%20%28single-precision%29))
  (Utilities|FlowControl|Delay 2.0)
  (if (not (Variables|Default|GetIsMoving))
    (Variables|Default|SetIsMoving true)
    (AI|AIMoveTo self (.RandomLocation (AI|Navigation|GetRandomReachablePointinRadius (Transformation|GetActorLocation) 1e+03 0 0)) 0 5.0 false
      (:OnSuccess
        _)
      (:OnFail
        _))
    (Variables|Default|SetIsMoving false)))

(fn ConstructionScript)

(fn TakeDamage
  (Effects|SpawnEmitteratLocation "/Game/InfinityBladeEffects/Effects/FX_Monsters/FX_Monster_Gruntling/Bomber/P_FireBombExplosion.P_FireBombExplosion" (Transformation|GetActorLocation)))

(fn Death
  (Game|SpawnActorfromClass "/Game/SimpleInventoryComponent/Blueprints/Actors/Chest/Examples/BP_Loot.BP_Loot_C" (Math|Transform|MakeTransform (Transformation|GetSocketLocation (Variables|Character|GetMesh) "Toes_L")) "Undefined" 0 3 1 0 0)
  (Actor|DestroyActor))