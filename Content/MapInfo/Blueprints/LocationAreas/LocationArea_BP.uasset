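; LocationArea_BP is a discoverable map area that marks a fast travel location as found when the player enters its radius.
; On BeginPlay it restores its LocationInfo from the SGK game instance's location list if a fast travel save exists.
; On first overlap it briefly shows a discovery widget with the enum-derived name, appends the found location to that list and saves.
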(event OnComponentBeginOverlap(AreaRadius)
  (params (OverlappedComponent :type Primitive%20Component%20Object%20Reference) (OtherActor :type Actor%20Object%20Reference) (OtherComp :type Primitive%20Component%20Object%20Reference) (OtherBodyIndex :type Integer) (bFromSweep :type Boolean) (SweepResult :type Hit%20Result%20Structure%20%28by%20ref%29))
  (bind _gameinstanceref (Variables|Default|GetGameInstanceRef))
  (if (== OtherActor (Game|GetPlayerCharacter 0))
    ;[0.096 1 0] Creates a Widget On Screen That Notifies The Player They Have Found A New Area / Does Only Once Per Area Found then removes it from screen
    (if (not (.LocationFound? (Utilities|Struct|BreakS_FTLocations (Variables|Default|GetLocationInfo))))
      (bind _returnvalue (UserInterface|CreateWidget "/Game/MapInfo/Widgets/NewLocationFound_WBP.NewLocationFound_WBP_C"))
      (UserInterface|Viewport|AddtoViewport _returnvalue 0)
      (Rendering|Components|TextRender|SetText (Variables|/Game/MapInfo/Widgets/NewLocationFound_WBP.NewLocationFound_WBP_C|GetLocationNameText _returnvalue) (Utilities|Text|ToText(String) (Utilities|String|EnumtoString (.Location (Utilities|Struct|BreakS_FTLocations (Variables|Default|GetLocationInfo))))))
      (bind _output_get (Variables|Default|SetLocationInfo (Utilities|Struct|MakeS_FTLocations (.Location (Utilities|Struct|BreakS_FTLocations (Variables|Default|GetLocationInfo))) true)))
      ;[0.096 1 0] On Begin Overlap : Gets the Location Area info and sends it to the Travel Widget when marker is found
      (Utilities|Array|Add (Variables|/Game/SurvivalGameKitV2/Blueprints/Saving/BP_SGKGameInstance.BP_SGKGameInstance_C|GetLocationAreaInfo _gameinstanceref) _output_get)
      ;[0.096 1 0] Save and remove from parent
      (Default|SaveFastTravelGame _gameinstanceref)
      (Utilities|FlowControl|Delay 3.0)
      (Widget|RemovefromParent _returnvalue))
    (else
      (Development|PrintString "Location Area: Player Character failed to overlap!" true true "(R=1.000000,G=0.000000,B=0.000000,A=1.000000)"))))

(event EventBeginPlay
  ;[0.096 1 0] Does Save Game Exist Check
  (bind _asbp_sgkgame_instance (Utilities|Casting|CastToBP_SGKGameInstance (Game|GetGameInstance)))
  (Variables|Default|SetGameInstanceRef _asbp_sgkgame_instance)
  (bind _returnvalue (SaveGame|DoesSaveGameExist "FastTravelSave"))
  (if _returnvalue
    (for _array_element (Variables|/Game/SurvivalGameKitV2/Blueprints/Saving/BP_SGKGameInstance.BP_SGKGameInstance_C|GetLocationAreaInfo (Variables|Default|GetGameInstanceRef))
      (if (Utilities|Enum|Equal(Enum) (.Location (Utilities|Struct|BreakS_FTLocations _array_element)) (.Location (Utilities|Struct|BreakS_FTLocations (Variables|Default|GetLocationInfo))))
        (Variables|Default|SetLocationInfo _array_element)))))

(fn ConstructionScript)