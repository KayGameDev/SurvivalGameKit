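; Level portal marker actor that activates when the player character enters its interaction area, as part of a fast travel system.
; Overlap shows the name widget, swaps the marker to its active material and sets ActivatePortal on the FastTravel_GI game instance.
; Leaving reverses these, then after a delay destroys the actor and clears DoesPortalAlreadyExist on the game instance.
; Re-entering does not cancel that pending destruction.
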(event OnComponentBeginOverlap(InteractionArea)
  (params (OverlappedComponent :type Primitive%20Component%20Object%20Reference) (OtherActor :type Actor%20Object%20Reference) (OtherComp :type Primitive%20Component%20Object%20Reference) (OtherBodyIndex :type Integer) (bFromSweep :type Boolean) (SweepResult :type Hit%20Result%20Structure%20%28by%20ref%29))
  ;[0.096 1 0] Displays the name (Over-head Text) of this portal marker when in interaction area and activates it. Hides the name when not in interaction area
  (if (== OtherActor (Game|GetPlayerCharacter 0))
    (Rendering|SetVisibility (Variables|Default|GetPortalWidget) true false)
    (bind _asfast_travel_gi (Utilities|Casting|CastToFastTravel_GI (Game|GetGameInstance)))
    (Variables|/Game/SimpleFastTravelSystem/Blueprints/FastTravel_GI.FastTravel_GI_C|SetActivatePortal _asfast_travel_gi true)
    ;[0.096 1 0] Changes The Color Of The Marker When Active / Not Active
    (Rendering|Material|SetMaterial (Variables|Default|GetMarker) 0 "/Game/SimpleFastTravelSystem/Materials/M_PortalActive.M_PortalActive")
    (else
      (Development|PrintString "Level Portal: Character failed to overlap!" true true "(R=1.000000,G=0.000000,B=0.000000,A=1.000000)"))))

(event OnComponentEndOverlap(InteractionArea)
  (params (OverlappedComponent :type Primitive%20Component%20Object%20Reference) (OtherActor :type Actor%20Object%20Reference) (OtherComp :type Primitive%20Component%20Object%20Reference) (OtherBodyIndex :type Integer))
  ;[0.096 1 0] Displays the name (Over-head Text) of this portal marker when in interaction area and activates it. Hides the name when not in interaction area
  (if (== OtherActor (Game|GetPlayerCharacter 0))
    (Rendering|SetVisibility (Variables|Default|GetPortalWidget) false false)
    (bind _asfast_travel_gi (Utilities|Casting|CastToFastTravel_GI (Game|GetGameInstance)))
    (Variables|/Game/SimpleFastTravelSystem/Blueprints/FastTravel_GI.FastTravel_GI_C|SetActivatePortal _asfast_travel_gi false)
    ;[0.096 1 0] Changes The Color Of The Marker When Active / Not Active
    (Rendering|Material|SetMaterial (Variables|Default|GetMarker) 0 "/Game/SimpleFastTravelSystem/Materials/M_PortalNotActive.M_PortalNotActive")
    ;[0.096 1 0] Destroys This Actor After A Certain Time
    (Utilities|FlowControl|Delay 1e+01)
    (Actor|DestroyActor)
    (Variables|/Game/SimpleFastTravelSystem/Blueprints/FastTravel_GI.FastTravel_GI_C|SetDoesPortalAlreadyExist _asfast_travel_gi false)))

(fn ConstructionScript)