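; Travel marker actor that the player discovers by walking into its interaction area, registering it for fast travel.
; On BeginPlay it restores its info from the game instance's TravelMarkerInfo array if the FastTravelSave slot exists.
; Each player overlap marks it found, stores its SpawnLocation transform, appends it to that array without checking for duplicates, and saves.
; Leaving hides the overhead name text; the commented notify widget display is absent.
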(event OnComponentBeginOverlap(InteractionArea)
  (params (OverlappedComponent :type Primitive%20Component%20Object%20Reference) (OtherActor :type Actor%20Object%20Reference) (OtherComp :type Primitive%20Component%20Object%20Reference) (OtherBodyIndex :type Integer) (bFromSweep :type Boolean) (SweepResult :type Hit%20Result%20Structure%20%28by%20ref%29))
  (bind _gameinstanceref (Variables|Default|GetGameInstanceRef))
  (bind _spawnlocation (Variables|Default|GetSpawnLocation))
  (if (== OtherActor (Game|GetPlayerCharacter 0))
    ;[0.096 1 0] Displays The Travel Marker Found Notify Widget / Does Only Once Per Marker Found then removes it from screen
    (bind _output_get (Variables|Default|SetMarkerInfo (Utilities|Struct|MakeS_FTMarkers (.TravelMarker (Utilities|Struct|BreakS_FTMarkers (Variables|Default|GetMarkerInfo))) (Transformation|GetWorldLocation _spawnlocation) (Transformation|GetWorldRotation _spawnlocation) true)))
    ;[0.096 1 0] Gets the Travel Marker info and sends it to the Game Instance when marker is found
    (Utilities|Array|Add (Variables|/Game/SurvivalGameKitV2/Blueprints/Saving/BP_SGKGameInstance.BP_SGKGameInstance_C|GetTravelMarkerInfo _gameinstanceref) _output_get)
    ;[0.096 1 0] Save and remove from parent
    (Default|SaveFastTravelGame _gameinstanceref)
    (Utilities|FlowControl|Delay 3.0)
    (else
      (Development|PrintString "Travel Marker: Character failed to overlap!" true true "(R=1.000000,G=0.000000,B=0.000000,A=1.000000)"))))

(event OnComponentEndOverlap(InteractionArea)
  (params (OverlappedComponent :type Primitive%20Component%20Object%20Reference) (OtherActor :type Actor%20Object%20Reference) (OtherComp :type Primitive%20Component%20Object%20Reference) (OtherBodyIndex :type Integer))
  (if (== OtherActor (Game|GetPlayerCharacter 0))
    ;[0.096 1 0] Displays the name (Over-head Text) of this marker when in interaction area and hides the name when not in interaction area
    (Rendering|SetVisibility (Variables|Default|GetMarkerNameText) false false)))

(event EventBeginPlay
  ;[0.096 1 0] Does Save Game Exist Check
  (bind _asbp_sgkgame_instance (Utilities|Casting|CastToBP_SGKGameInstance (Game|GetGameInstance)))
  (Variables|Default|SetGameInstanceRef _asbp_sgkgame_instance)
  (bind _returnvalue (SaveGame|DoesSaveGameExist "FastTravelSave"))
  (if _returnvalue
    (for _array_element (Variables|/Game/SurvivalGameKitV2/Blueprints/Saving/BP_SGKGameInstance.BP_SGKGameInstance_C|GetTravelMarkerInfo (Variables|Default|GetGameInstanceRef))
      (if (Utilities|Enum|Equal(Enum) (.TravelMarker (Utilities|Struct|BreakS_FTMarkers _array_element)) (.TravelMarker (Utilities|Struct|BreakS_FTMarkers (Variables|Default|GetMarkerInfo))))
        (Variables|Default|SetMarkerInfo _array_element)))))

(fn ConstructionScript)