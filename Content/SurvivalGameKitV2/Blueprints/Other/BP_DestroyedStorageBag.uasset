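; BP_DestroyedStorageBag is an interactable bag actor in Survival Game Kit V2 that holds an inventory, apparently for destroyed storage.
; It implements the SGK interaction functions, always allowing interaction and offering a single open-inventory action.
; Interact calls ServerOpenExtInv on the player's inventory to open the bag's BPMasterInventory as an external inventory.
; Item, drop, code-lock and player-verification functions are stubs returning false or empty values.
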(fn ConstructionScript)

(fn SGKAllowInteraction
  (return true))

(fn SGKCodeCheck
  (params (Code :type Text))
  (return false))

(fn SGKDropItem
  (params (InvItem :type S%20Inv%20Item%20Structure) (Dropped :type Boolean) (Spawned :type Boolean) (SaveLoaded :type Boolean))
  (return false))

(fn SGKEndInteraction
  (params (PlayerInventory :type BP%20Player%20Inventory%20Object%20Reference))
  (return false))

(fn SGKGetVerifiedPlayers
  (return 0))

(fn SGKInteract
  (params (PlayerInventory :type BP%20Player%20Inventory%20Object%20Reference) (Action :type E_WorldActions%20Enum :default "NewEnumerator0"))
  (Default|ServerOpenExtInv PlayerInventory (Variables|Default|GetBP_MasterInventory))
  (return true))

(fn SGKInteractName
  (return (Variables|Interaction|GetInteractName)))

(fn SGKInvItem
  (return false ""))

(fn SGKItemAmount
  (return 0))

(fn SGKMesh
  (return 0))

(fn SGKPossibleActions
  (params (PlayerInventory :type BP%20Player%20Inventory%20Object%20Reference))
  (return true (Utilities|Array|MakeArray (Utilities|Struct|MakeS_WorldAction "NewEnumerator3" (Variables|Interaction|GetOpenInventoryText)))))

(fn SGKUpdateCode
  (params (Code :type Text))
  (return false))

(fn SGKVerifyPlayer
  (params (Text :type Text))
  (return false))